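; Selectable Paper2D flipbook actor that the player claims by holding the scan input while the cursor hovers over it.
; The Highlight timeline fades a flipbook copy of the render component's sprite, reversing when hover or input stops, and fires Select from an event track.
; Select runs once, reporting crew status, alive status and attached messages to the Commlink player controller.
; Crew finds also cycle the music mix and activate the actor's audio.
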(event `self.ReceiveTick`
  (params (DeltaSeconds :type "Float (single-precision)"))
  (if (`self.isClaimed`)
    _
    (elif (and (`self.IsHovered`) (`self.IsMouseDown`))
      (bind (_direction _selection_opacity) (`Timeline|Highlight` :`NewTime` 2.0 :!label _label)
        (:`Update`
          (`PaperFlipbookComponent.SetSpriteColor` (`self.PaperFlipbook`) (make `LinearColor` 1.0 1.0 1.0 _selection_opacity)))
        (:`select`
          (`self.Select`)))
      (else
        (goto _label :!via `Reverse`)))))

(event `InputAction|scan` :consume false
  (params (Key :type "Key Structure"))
  (:`Pressed`
    (set `self.IsMouseDown` true))
  (:`Released`
    (set `self.IsMouseDown` false)))

(event `self.ReceiveActorBeginCursorOver`
  (set `self.IsHovered` true))

(event `self.ReceiveActorEndCursorOver`
  (set `self.IsHovered` false))

(fn `Select`
  (if (not (`self.isClaimed`))
    (set `self.isClaimed` true)
    (`|ExecutionSequence`
      (:`then_0`
        (bind _ascommlink_player_controller_bp (cast `/Game/Blueprints/CommlinkPlayerController_BP` (`GameplayStatics.GetPlayerController` 0))))
      (:`then_1`
        (if (`self.IsCrew`)
          (`/Game/Blueprints/CommlinkPlayerController_BP.Cycle Music Mix Index` _ascommlink_player_controller_bp)
          (`ActorComponent.Activate` (`self.Audio`) false)))
      (:`then_2`
        (`CommlinkPlayerController.AccountFind` _ascommlink_player_controller_bp self (`self.IsCrew`) (`self.IsAlive`) (`self.SelectionEntries`))))))

(fn `UserConstructionScript`
  (`PaperFlipbookComponent.SetFlipbook` (`self.PaperFlipbook`) (`PaperFlipbookComponent.GetFlipbook` (`self.RenderComponent`))))