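; Player controller for Commlink that moves the pawn across the world, drives the HUD and lets the player eavesdrop on recordings.
; Axis input feeds weighted moving averages, zeroed on sign changes, for smoothed swept movement that updates HUD coordinates.
; A toggle overrides the audio listener to the selected recording's position from EnvironmentalListener and relabels the HUD audio source.
; Other keys cycle recordings, HUD vision modes and a music mix parameter, or quit.
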(event `InputAxis|Vertical`
  (params (AxisValue :type "Float (single-precision)"))
  (`|ExecutionSequence`
    (:`then_0`
      (if (not (== (`KismetMathLibrary.SignOfFloat` AxisValue) (`KismetMathLibrary.SignOfFloat` (`self.MovingAvgVertical`))))
        (set `self.MovingAvgVertical` 0.0)))
    (:`then_1`
      (bind _output_get (set `self.MovingAvgVertical` (`KismetMathLibrary.WeightedMovingAverage_Float` (* (`self.Speed`) AxisValue (`self.deltaTime`)) (`self.MovingAvgVertical`) 0.01)))
      (`self.K2_AddActorWorldOffset` (`self.MyPawn`) (`KismetMathLibrary.MakeVector` _output_get) true false)
      (`self.Update Coords`))))

(event `InputAxis|horizontal`
  (params (AxisValue :type "Float (single-precision)"))
  (`|ExecutionSequence`
    (:`then_0`
      (if (not (== (`KismetMathLibrary.SignOfFloat` AxisValue) (`KismetMathLibrary.SignOfFloat` (`self.MovingAvgHorizontal`))))
        (set `self.MovingAvgHorizontal` 0.0)))
    (:`then_1`
      (bind _output_get (set `self.MovingAvgHorizontal` (`KismetMathLibrary.WeightedMovingAverage_Float` (* AxisValue (`self.Speed`) (`self.deltaTime`)) (`self.MovingAvgHorizontal`) 0.01)))
      (`self.K2_AddActorWorldOffset` (`self.MyPawn`) (`KismetMathLibrary.MakeVector` 0.0 _output_get) true false)
      (`self.Update Coords`))))

(event `self.ReceiveTick`
  (params (DeltaSeconds :type "Float (single-precision)"))
  (set `self.deltaTime` DeltaSeconds))

(event `Key|Escape`
  (params (Key :type "Key Structure"))
  (:`Pressed`
    (`KismetSystemLibrary.QuitGame` null "Quit")))

(event `Key|E`
  (params (Key :type "Key Structure"))
  (:`Pressed`
    (`self.CycleRecording`)))

(event `Key|Q`
  (params (Key :type "Key Structure"))
  (:`Pressed`
    (`/Engine/EditorBlueprintResources/StandardMacros.FlipFlop`
      (:`A`
        (`self.Begin Listen Recording`))
      (:`B`
        (`self.End Listen Recording`)))))

(event `Key|F`
  (params (Key :type "Key Structure"))
  (:`Pressed`
    (`self.Cycle Vision Mode`)))

(event `Begin Listen Recording`
  (set `self.IsListeningToRecording` true)
  (`self.SetAudioListenerOverride` null (`CommlinkSoundRecordingListener.GetListenerLocation` (`self.EnvironmentalListener`) (`self.RecordingIndex`)))
  (`self.SetAudioUI`))

(event `Key|V`
  (params (Key :type "Key Structure"))
  (:`Pressed`
    (`self.Cycle Music Mix Index`)))

(event `End Listen Recording`
  (set `self.IsListeningToRecording` false)
  (`self.ClearAudioListenerOverride`)
  (`self.SetAudioUI`))

(event `Cycle Vision Mode`
  (bind _result (`/Engine/EditorBlueprintResources/StandardMacros.IncrementInt` (`self.Vision Index`))
    (:`  `
      (bind _output_get (set `self.Vision Index` (mod _result 3)))
      (`/Game/HUD/CommlinkHUD.Set Vision Type` (`self.My Hud`) _output_get))))

(event `Cycle Music Mix Index`
  (bind _result (`/Engine/EditorBlueprintResources/StandardMacros.IncrementInt` (`self.Music Mix Index`))
    (:`  `
      (bind _output_get (set `self.Music Mix Index` (mod _result 9)))
      (`self.Set Music Index` _output_get))))

(fn `Set Audio UI`)

(fn `Set Music Index`
  (params (MixRatio :type Integer))
  (`AudioComponent.SetFloatParameter` (`self.Audio`) "MixParam" (* MixRatio 0.1)))

(fn `SetAudioUI`
  (if (`self.IsListeningToRecording`)
    (`/Game/HUD/CommlinkHUD.Set Audio Info` (`self.My Hud`) (`|FormatText` "Person {int}" (`self.RecordingIndex`)) "SUIT AUDIO:")
    (else
      (`/Game/HUD/CommlinkHUD.Set Audio Info` (`self.My Hud`) "" "LOCAL AUDIO"))))

(fn `Update Coords`
  (bind (_returnvalue_x _returnvalue_y) (`KismetMathLibrary.BreakVector` (+ (* (`self.K2_GetActorLocation` (`self.MyPawn`)) 0.2) (2000.0 7000.0 0.0))))
  (`/Game/HUD/CommlinkHUD.Set Coords` (`self.My Hud`) (`KismetMathLibrary.Round` _returnvalue_y) (`KismetMathLibrary.Round` _returnvalue_x)))

(fn `UserConstructionScript`
  (`self.Set Music Index` 0))