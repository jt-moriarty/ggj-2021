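; Commlink sound listener actor that switches which of the game mode's recorded or in-world audio channels is heard.
; Construction copies AudioInfos from CommlinkGameMode_BP, creating a muted audio component per non-world cue and an empty slot for in-world ones, then unmutes the first.
; SetListenIndex switches by volume alone, unmuting the chosen component and silencing the rest.
; GetListenerLocation returns the listening actor's position for in-world entries, otherwise its own.
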(fn `Get Listener Location`
  (params (Index :type Integer))
  (returns (ListenerPosition :type "Vector Structure"))
  (bind (_output_isinworld _output_listeningactor) (break `CommlinkAudioSourceInfo` (`|GetArrayItem` (`self.AudioInfos`) Index)))
  (if _output_isinworld
    (return (`self.K2_GetActorLocation` _output_listeningactor))
    (else
      (return (`self.K2_GetActorLocation`)))))

(fn `Set Listen Index`
  (params (CueIndex :type Integer))
  (for (_array_element _array_index) (`self.MyAudioComponents`)
    (`/Engine/EditorBlueprintResources/StandardMacros.IsValid` _array_element
      (:`Is Valid`
        (if (== _array_index CueIndex)
          (`AudioComponent.SetVolumeMultiplier` _array_element 1.0)
          (else
            (`AudioComponent.SetVolumeMultiplier` _array_element 0.0)))))))

(fn `UserConstructionScript`
  (bind _ascommlink_game_mode_bp (cast `/Game/Blueprints/CommlinkGameMode_BP` (`GameplayStatics.GetGameMode`)))
  (bind _output_get (set `self.AudioInfos` (`/Game/Blueprints/CommlinkGameMode_BP.Audio Infos` _ascommlink_game_mode_bp)))
  (for _array_element _output_get
    (bind (_isinworld _listeningactor _soundcue) (break `CommlinkAudioSourceInfo` _array_element))
    (if _isinworld
      (`KismetArrayLibrary.Array_Add` (`self.MyAudioComponents`))
      (else
        (bind _returnvalue (`AddComponent|NODE_AddAudioComponent-0`))
        (`AudioComponent.SetSound` _returnvalue _soundcue)
        (`AudioComponent.SetVolumeMultiplier` _returnvalue 0.0)
        (`KismetArrayLibrary.Array_Add` (`self.MyAudioComponents`) _returnvalue))))
  (`AudioComponent.SetVolumeMultiplier` (`|GetArrayItem` (`self.MyAudioComponents`)) 1.0))