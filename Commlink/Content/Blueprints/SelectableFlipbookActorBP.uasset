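; A selectable flipbook actor that the player selects by holding the scan input while the cursor hovers over it.
; An overlay flipbook copies the actor's flipbook at construction, and the Highlight timeline drives its opacity.
; Until the actor is claimed, the timeline plays while hovered and held, fires Select from its event track, and reverses otherwise.
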(event `self.ReceiveTick`
  (params (DeltaSeconds :type "Float (single-precision)"))
  (if (`self.IsClaimed`)
    _
    (elif (and (`self.IsHovered`) (`self.IsMouseDown`))
      (bind (_direction _selection_opacity) (`Timeline|Highlight` :`NewTime` 2.0 :!label _label)
        (:`Update`
          (`PaperFlipbookComponent.SetSpriteColor` (`self.OverlayFlipbook`) (make `LinearColor` 1.0 1.0 1.0 _selection_opacity)))
        (:`select`
          (`self.Select`)))
      (else
        (goto _label :!via `Reverse`)))))

(event `InputAction|scan` :consume false
  (params (Key :type "Key Structure"))
  (:`Pressed`
    (set `self.IsMouseDown` true))
  (:`Released`
    (set `self.IsMouseDown` false)))

(event `self.ReceiveActorBeginCursorOver`
  (set `self.IsHovered` true))

(event `self.ReceiveActorEndCursorOver`
  (set `self.IsHovered` false))

(fn `UserConstructionScript`
  (`PaperFlipbookComponent.SetFlipbook` (`self.OverlayFlipbook`) (`PaperFlipbookComponent.GetFlipbook` (`self.RenderComponent`))))