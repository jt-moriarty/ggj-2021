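; CommlinkHUDBP is the HUD Blueprint that owns the main on-screen widget and exposes it to the rest of the game.
; On BeginPlay it creates WidgetHUD, adds it to the viewport, registers itself with the Commlink player controller and triggers that controller's audio UI setup.
; Its events and functions relay coordinates, vision type, audio source details, report-submission notices and pending message lines to the widget.
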(event `self.ReceiveBeginPlay`
  (bind _returnvalue (`|CreateWidget` "/Game/HUD/WidgetHUD.WidgetHUD_C"))
  (`UserWidget.AddToViewport` _returnvalue 0)
  (set `self.Main HUD Widget` _returnvalue)
  (bind _ascommlink_player_controller_bp (cast `/Game/Blueprints/CommlinkPlayerController_BP` (`GameplayStatics.GetPlayerController` 0)))
  (set `/Game/Blueprints/CommlinkPlayerController_BP.My Hud` self _ascommlink_player_controller_bp)
  (`CommlinkPlayerController.SetAudioUI` _ascommlink_player_controller_bp))

(event `self.SetCoords`
  (params (XCoord :type Integer) (YCoord :type Integer))
  (bind _coordswidget (`/Game/HUD/WidgetHUD.CoordsWidget` (`self.Main HUD Widget`)))
  (set `/Game/HUD/CoordsWidget.XCoord` XCoord _coordswidget)
  (set `/Game/HUD/CoordsWidget.YCoord` YCoord _coordswidget))

(event `self.SetVisionType`
  (params (VisionIndex :type Integer))
  (`/Game/HUD/WidgetHUD.SetVisionType` (`self.Main HUD Widget`) VisionIndex))

(fn `OnMaySubmitReport`
  (`/Game/HUD/WidgetHUD.OnMaySubmitReport` (`self.Main HUD Widget`)))

(fn `SendMessage`
  (params (Message :type Text))
  (`/Game/HUD/WidgetHUD.Add Pending Line` (`self.Main HUD Widget`) Message))

(fn `Set Audio Info`
  (params (SourceName :type Text) (SourceType :type Text))
  (`/Game/HUD/WidgetHUD.SetAudioSourceDetails` (`self.Main HUD Widget`) SourceName SourceType))

(fn `UserConstructionScript`)